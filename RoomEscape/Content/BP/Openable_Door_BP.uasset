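; Openable door actor that swings open and closed in response to requests from its OpenDoor event source.
; On begin play it caches its initial rotation and location.
; An open request plays a timeline whose angle curve is added as yaw to the initial rotation, and a close request reverses it.
; A timeline event track plays the door sound at the initial location.
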(event `self.ReceiveBeginPlay`
  (set `self.Initial Rotation` (`self.K2_GetActorRotation`))
  (set `self.Initial Location` (`self.K2_GetActorLocation`)))

(event `self.OpenDoor.OnOpenRequest`
  (bind (_direction _open_angle) (`Timeline|Timeline_0` :!label _label)
    (:`Update`
      (`self.K2_SetActorRotation` (`KismetMathLibrary.ComposeRotators` (`self.Initial Rotation`) (`KismetMathLibrary.MakeRotator` 0.0 0.0 _open_angle))))
    (:`Sound Timing`
      (`GameplayStatics.PlaySoundAtLocation` "/Game/Sounds/close_door_1.close_door_1" (`self.Initial Location`) (struct) 1.0 1.0 0.0 null null self))))

(event `self.OpenDoor.OnCloseRequest`
  (goto _label :!via `Reverse`))

(fn `UserConstructionScript`)